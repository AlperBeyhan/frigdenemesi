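; Main character Blueprint in runman that patrols a looping route of waypoint actors on its own.
; On BeginPlay, FallowWaypoint uses AIMoveTo to send the pawn to the current entry in the Waypoints array.
; Each successful move advances the index, wraps to zero after the last entry, and re-triggers the event after a short delay.
; Only the success output is wired, so a failed move stops the patrol.
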(event `self.ReceiveBeginPlay`
  (`self.Fallow Waypoint`))

(event `Fallow Waypoint`
  (`|AIMoveTo` self (0.0 0.0 0.0) (`|GetArrayItem` (`self.Waypoints`) (`self.current Waypoint`))
    (:`then`
      (`/Engine/EditorBlueprintResources/StandardMacros.IncrementInt` (`self.current Waypoint`)
        (:`  `
          (if (>= (`self.current Waypoint`) (`KismetArrayLibrary.Array_Length` (`self.Waypoints`)))
            (set `self.current Waypoint` 0))
          (`KismetSystemLibrary.Delay` 0.2)
          (`self.Fallow Waypoint`))))))

(fn `UserConstructionScript`)